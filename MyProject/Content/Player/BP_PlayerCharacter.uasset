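; Player character Blueprint that shows the score HUD and takes damage on contact.
; On BeginPlay it creates the Score widget for player 0 and adds it to the viewport.
; Any capsule overlap, with no actor filtering, calls OnDamaged, which has the HealthComponent update health.
; Unconnected nodes for opening the testing-ground level and resetting the EndlessGameMode never run.
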(event `self.ReceiveBeginPlay`
  (bind _returnvalue (`|CreateWidget` "/Game/UI/Widget_Score.Widget_Score_C" (`GameplayStatics.GetPlayerController` 0)))
  (bind _output_get (set `self.ScoreWidget` _returnvalue))
  (`UserWidget.AddToViewport` _output_get 0))

(event `self.Capsule.OnComponentBeginOverlap`
  (params (OverlappedComponent :type "PrimitiveComponent Object Reference") (OtherActor :type "Actor Object Reference") (OtherComp :type "PrimitiveComponent Object Reference") (OtherBodyIndex :type Integer) (bFromSweep :type Boolean) (SweepResult :type "HitResult Structure (by ref)"))
  (`self.OnDamaged`))

(event `OnDamaged`
  (`HealthComponent.UpdateHealth` (`self.Health Component`)))

(fn `UserConstructionScript`)